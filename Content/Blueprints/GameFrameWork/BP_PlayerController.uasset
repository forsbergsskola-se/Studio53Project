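; BP_PlayerController is a player controller that turns movement, turning and jump input into actions on the controlled pawn.
; Move axes add movement input along the pawn's forward and right vectors, while mouse and gamepad turn axes add controller yaw, each scaled by its own sensitivity variable.
; Jump casts the pawn to Character and prints an unsupported-pawn message if the cast fails.
; It handles no pitch input.
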(event EventBeginPlay)

(event EventTick
  (params (DeltaSeconds :type Float%20%28single-precision%29)))

(event Input|ActionEvents|InputActionJump
  (params (Key :type Key%20Structure :default "None"))
  (:Pressed
    (bind _ascharacter (Utilities|Casting|CastToCharacter (Pawn|GetControlledPawn))
      (:then
        (Character|Jump _ascharacter))
      (:CastFailed
        (Development|PrintString "Only BP_PlayerCharacter is Supported")))))

(event Input|AxisEvents|InputAxisMoveForward/Backward
  (params (AxisValue :type Float%20%28single-precision%29))
  (bind _returnvalue (Pawn|GetControlledPawn))
  (Pawn|Input|AddMovementInput _returnvalue (Transformation|GetActorForwardVector _returnvalue) AxisValue false))

(event Input|AxisEvents|InputAxisMoveRight/Left
  (params (AxisValue :type Float%20%28single-precision%29))
  (bind _returnvalue (Pawn|GetControlledPawn))
  (Pawn|Input|AddMovementInput _returnvalue (Transformation|GetActorRightVector _returnvalue) AxisValue false))

(event Input|AxisEvents|InputAxisTurnRight/LeftGamepad
  (params (AxisValue :type Float%20%28single-precision%29))
  (Pawn|Input|AddControllerYawInput (Pawn|GetControlledPawn) (* AxisValue (Variables|Default|GetGame%20Pad%20Sensitivity%20X))))

(event Input|AxisEvents|InputAxisTurnRight/LeftMouse
  (params (AxisValue :type Float%20%28single-precision%29))
  (Pawn|Input|AddControllerYawInput (Pawn|GetControlledPawn) (* AxisValue (Variables|Default|GetMouse%20Sensitivity%20X))))

(fn ConstructionScript)