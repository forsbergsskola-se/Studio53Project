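; Player controller that turns movement, look and jump input into actions on the controlled pawn.
; Movement follows control rotation, and jump requires a BP_PlayerCharacter, printing a message otherwise.
; Look input feeds controller yaw and pitch, with sensitivity scaling on mouse yaw only and frame-time-scaled rates for gamepad.
; Gamepad yaw has two handlers on the same axis, one sensitivity-scaled and one frame-time-scaled.
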(event EventBeginPlay)

(event EventTick
  (params (DeltaSeconds :type Float%20%28single-precision%29)))

(event Input|ActionEvents|InputActionJump
  (params (Key :type Key%20Structure :default "None"))
  (:Pressed
    (bind _asbp_player_character (Utilities|Casting|CastToBP_PlayerCharacter (Pawn|GetControlledPawn))
      (:then
        (Character|Jump _asbp_player_character))
      (:CastFailed
        (Development|PrintString "Only BP_PlayerCharacter is Supported")))))

(event Input|AxisEvents|InputAxisTurnRight/LeftGamepad
  (params (AxisValue :type Float%20%28single-precision%29))
  (Pawn|Input|AddControllerYawInput (Pawn|GetControlledPawn) (* AxisValue (Variables|Default|GetTurn%20Rate%20Gamepad) (Utilities|Time|GetWorldDeltaSeconds))))

(event Input|AxisEvents|InputAxisLookUp/DownMouse
  (params (AxisValue :type Float%20%28single-precision%29))
  (Pawn|Input|AddControllerPitchInput (Pawn|GetControlledPawn) AxisValue))

(event Input|AxisEvents|InputAxisLookUp/DownGamepad
  (params (AxisValue :type Float%20%28single-precision%29))
  (Pawn|Input|AddControllerPitchInput (Pawn|GetControlledPawn) (* AxisValue (Variables|Default|GetTurn%20Rate%20Gamepad) (Utilities|Time|GetWorldDeltaSeconds))))

(event Input|AxisEvents|InputAxisTurnRight/LeftGamepad
  (params (AxisValue :type Float%20%28single-precision%29))
  (Pawn|Input|AddControllerYawInput (Pawn|GetControlledPawn) (* AxisValue (Variables|Default|GetGame%20Pad%20Sensitivity%20X))))

(event Input|AxisEvents|InputAxisTurnRight/LeftMouse
  (params (AxisValue :type Float%20%28single-precision%29))
  (Pawn|Input|AddControllerYawInput (Pawn|GetControlledPawn) (* AxisValue (Variables|Default|GetMouse%20Sensitivity%20X))))

(event Input|AxisEvents|InputAxisMoveForward/Backward
  (params (AxisValue :type Float%20%28single-precision%29))
  (Pawn|Input|AddMovementInput (Pawn|GetControlledPawn) (Math|Vector|GetForwardVector (Math|Rotator|MakeRotator 0.0 0.0 (.yaw (Pawn|GetControlRotation :!class /Script/Engine.Controller)))) AxisValue false))

(event Input|AxisEvents|InputAxisMoveRight/Left
  (params (AxisValue :type Float%20%28single-precision%29))
  (bind _returnvalue (Pawn|GetControlRotation :!class /Script/Engine.Controller))
  (Pawn|Input|AddMovementInput (Pawn|GetControlledPawn) (Math|Vector|GetRightVector (Math|Rotator|MakeRotator (.roll _returnvalue) 0.0 (.yaw _returnvalue))) AxisValue false))

(fn ConstructionScript)