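; Player character Blueprint with a short-range blink teleport and an interact input for opening doors.
; Teleport line-traces forward from the Sphere component, then moves the player to the hit point, or to the trace's end if nothing is hit.
; Timelines narrow the camera FOV before the jump and restore it afterward.
; OpenDoor sends an Interact message to the first overlapping actor implementing InteractInterface.
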(event EventBeginPlay)

(event Collision|EventActorBeginOverlap
  (params (OtherActor :type Actor%20Object%20Reference)))

(event EventTick
  (params (DeltaSeconds :type Float%20%28single-precision%29)))

(event Input|ActionEvents|InputActionOpenDoor
  (params (Key :type Key%20Structure :default "None"))
  ;[1 1 1] Open Doors
  (:Pressed
    (bind _array_element (Utilities|Array|ForEachLoopwithBreak (Collision|GetOverlappingActors 0 :!class /Script/Engine.Actor) :!label _label)
      (:LoopBody
        (if (Utilities|DoesObjectImplementInterface _array_element "/Game/_GENERATED/Blueprints/InteractInterface.InteractInterface_C")
          (Class|InteractInterface|Interact(Message) _array_element self)
          (goto _label Break))))))

(event Input|ActionEvents|InputActionTeleportation
  (params (Key :type Key%20Structure :default "None"))
  (bind _outrotation (Actor|GetActorEyesViewPoint))
  (bind _sphere (Variables|Default|GetSphere))
  (bind _returnvalue (Math|Vector|GetForwardVector _sphere))
  (bind _returnvalue_2 (Transformation|GetWorldLocation _sphere))
  (bind _returnvalue_3 (* _returnvalue 5e+02))
  (bind _returnvalue_4 (+ _returnvalue_2 _returnvalue_3))
  (:Pressed
    (bind (_outhit _returnvalue_5) (Collision|LineTraceByChannel _returnvalue_2 _returnvalue_4 "TraceTypeQuery1" true 0 "ForDuration"))
    (if _returnvalue_5
      (bind _alpha (Timeline|Teleport PlayFromStart)
        (:Update
          (Camera|SetFieldOfView (Variables|Default|GetCamera) (Math|Float|Lerp 9e+01 6e+01 _alpha)))
        (:Finished
          (Transformation|Teleport (.Location (Collision|BreakHitResult _outhit)) _outrotation)
          (bind _alpha_2 (Timeline|Timeline_0 ReverseFromEnd)
            (:Update
              (Camera|SetFieldOfView (Variables|Default|GetCamera) (Math|Float|Lerp 9e+01 6e+01 _alpha_2))))))
      (else
        (bind _alpha_3 (Timeline|Timeline_1 PlayFromStart)
          (:Update
            (Camera|SetFieldOfView (Variables|Default|GetCamera) (Math|Float|Lerp 9e+01 6e+01 _alpha_3)))
          (:Finished
            (Transformation|Teleport _returnvalue_4 _outrotation)
            (bind _alpha_4 (Timeline|Timeline_2 ReverseFromEnd)
              (:Update
                (Camera|SetFieldOfView (Variables|Default|GetCamera) (Math|Float|Lerp 9e+01 6e+01 _alpha_4))))))))))

(fn ConstructionScript)