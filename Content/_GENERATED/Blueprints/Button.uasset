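; An interactable button that opens matching SwitchDoor actors once a switch requirement in the game mode is met.
; On Interact, it looks up KeyToFind in the BP_GameMode Switches map and checks that the value reaches RequiredSwitchValue.
; It then searches all SwitchDoor actors for a DoorValue equal to its ButtonValue, opens each match and switches the first player controller's view target to that door.
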(event EventInteract
  (params (Player :type BP%20Player%20Character%20Object%20Reference))
  (bind _asbp_game_mode (Utilities|Casting|CastToBP_GameMode (Game|GetGameMode)))
  (if (.ReturnValue (Utilities|Map|Find (Variables|/Game/_GENERATED/Blueprints/BP_GameMode.BP_GameMode_C|GetSwitches _asbp_game_mode) (Variables|Default|GetKey%20to%20find)))
    (if (>= (.Value (Utilities|Map|Find (Variables|/Game/_GENERATED/Blueprints/BP_GameMode.BP_GameMode_C|GetSwitches _asbp_game_mode) (Variables|Default|GetKey%20to%20find))) (Variables|Default|GetRequired%20Switch%20Value))
      (bind _outactors (Actor|GetAllActorsOfClass "/Game/_GENERATED/Blueprints/SwitchDoor.SwitchDoor_C"))
      (bind _array_element (Utilities|Array|ForEachLoopwithBreak _outactors)
        (:LoopBody
          (if (== (Variables|/Game/_GENERATED/Blueprints/SwitchDoor.SwitchDoor_C|GetDoor%20Value _array_element) (Variables|Default|GetButton%20Value))
            (Default|OpenDoor _array_element Player)
            (Game|Player|SetViewTargetwithBlend (Game|GetPlayerController 0) _array_element 0.0 "VTBlend_Linear" 0.0 false)))))))

(fn ConstructionScript)